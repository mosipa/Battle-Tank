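; Mortar Blueprint that sets up an aimable mortar emplacement with a health bar widget.
; On BeginPlay it initialises its TankAiming component with the Barrel and Dome, the dome acting as the turret.
; It then casts its widget component's user widget to HealthBar_BP and assigns itself as that widget's Tank, reusing the tank health bar.
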(event `self.ReceiveBeginPlay`
  (`TankAimingComponent.Initialise` (`self.TankAiming`) (`self.Barrel`) (`self.Dome`))
  (`self.Initialise HealthBar Widget`))

(fn `Initialise HealthBar Widget`
  (bind _ashealth_bar_bp (cast `/Game/Blueprints/UI/HealthBar_BP` (`WidgetComponent.GetUserWidgetObject` (`self.Widget`))))
  (set `/Game/Blueprints/UI/HealthBar_BP.Tank` self _ashealth_bar_bp))

(fn `UserConstructionScript`)